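; BP_ElectricPanel is an electric panel meant to activate once the player has hit it enough times.
; BeginPlay creates a dynamic material instance on the panel mesh and tints it gray.
; HitbyPlayer compares CurrentHits to MaxHits, then latches IsActivated, turns the panel green and shows its light.
; The CurrentHits increment node sits off the execution path, so the hit count is not incremented as wired.
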(event EventBeginPlay
  (bind _returnvalue (Rendering|Material|CreateDynamicMaterialInstance (Variables|Default|GetPanelMesh) 0 0 "None" :!class /Script/Engine.PrimitiveComponent))
  (bind _output_get (Variables|Default|SetDynamicMat _returnvalue))
  (Rendering|Material|SetVectorParameterValue _output_get "PanelColor" (Class|KismetMathLibrary|LinearColorGray) :!class /Script/Engine.MaterialInstanceDynamic))

(event EventHitbyPlayer
  (params (Damage :type Float%20%28double-precision%29))
  (Development|PrintText "hit by player")
  (if (not (Variables|Default|GetbIsActivated))
    (Variables|Default|SetCurrentHits (stale _result))
    (if (>= (Variables|Default|GetCurrentHits) (Variables|Default|GetMaxHits))
      (Variables|Default|SetbIsActivated true)
      (Rendering|Material|SetVectorParameterValue (Variables|Default|GetDynamicMat) "PanelColor" (Utilities|Struct|MakeLinearColor 0.0 1.0 0.0 0.0) :!class /Script/Engine.MaterialInstanceDynamic)
      (Rendering|SetVisibility (Variables|Default|GetPanelLight) true false))))

(fn ConstructionScript)